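; Collectible coin interactable that spins in place and adds a coin to the player when picked up.
; Tick rotates the Coin component around its roll axis at a rate set by RotationSpeed, scaled by frame time.
; Interact casts the first player pawn to ThirdPersonCharacter, calls AddCoin on it, prints a debug message and destroys the coin.
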(event EventTick
  (params (DeltaSeconds :type Float%20%28single-precision%29))
  (bind _coin (Variables|Default|GetCoin))
  (bind _relativerotation (Variables|/Script/Engine.SceneComponent|GetRelativeRotation _coin))
  (Transformation|SetRelativeRotation _coin (Math|Rotator|MakeRotator (+ (.roll _relativerotation) (* DeltaSeconds (Variables|Default|GetRotationSpeed) 1e+02)) (.pitch _relativerotation) (.yaw _relativerotation)) false false))

(event EventInteract
  (bind _asthird_person_character (Utilities|Casting|CastToThirdPersonCharacter (Game|Player|GetPlayerPawn 0)))
  (Default|AddCoin _asthird_person_character)
  (Development|PrintString "PickedCoin")
  (Actor|DestroyActor))

(fn ConstructionScript)